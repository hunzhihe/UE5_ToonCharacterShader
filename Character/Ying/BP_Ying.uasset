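; BP_Ying is the Ying character Blueprint that feeds light direction relative to the character into SDF-based rendering.
; It compares the SDF_Light-tagged directional light's forward vector with the DEF-spine_006 socket's, using cross and dot products to derive an offset, zero on one side.
; The SDFMapped curve remaps that offset into MPC_Render's SDF_Location.
; Updates run on Tick and through a looping timer started by the construction script.
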(event `SDF更新`
  (bind _returnvalue (`KismetMathLibrary.GetForwardVector` (`SceneComponent.GetSocketRotation` (`self.Mesh`) "DEF-spine_006")))
  (bind _outactors (`GameplayStatics.GetAllActorsOfClassWithTag` "/Script/Engine.DirectionalLight" "SDF_Light" :!label _label))
  (bind _output_get (set `self.Light` (`|GetArrayItem` _outactors)))
  (`/Engine/EditorBlueprintResources/StandardMacros.IsValid` _output_get
    (:`Is Valid`
      (bind _returnvalue_2 (`KismetMathLibrary.GetForwardVector` (`self.K2_GetActorRotation` _output_get)))
      (bind (_returnvalue_x _returnvalue_y _returnvalue_z) (`KismetMathLibrary.BreakVector` (`KismetMathLibrary.Cross_VectorVector` _returnvalue_2 _returnvalue)))
      (if (<= _returnvalue_z 0.0)
        (bind _returnvalue_3 (`KismetMathLibrary.Dot_VectorVector` _returnvalue_2 _returnvalue))
        (if (<= _returnvalue_3 0.0)
          (set `self.SDF_Offest` (/ (- -2.0 _returnvalue_3) -2.0))
          (else
            (set `self.SDF_Offest` (/ (+ (- 1.0 _returnvalue_3) 1.0) -2.0))))
        (else
          (set `self.SDF_Offest` 0.0)))
      (`KismetMaterialLibrary.SetScalarParameterValue` "/Game/ToonCharacter/Stage/Materials/MaterialTools/MPC_Render.MPC_Render" "SDF_Location" (`CurveFloat.GetFloatValue` (`self.SDF_Mapped`) (`self.SDF_Offest`))))))

(event `Start Calculate SDF`
  (`|ExecutionSequence`
    (:`then_0`
      (goto _label))
    (:`then_1`
      (bind _returnvalue (`KismetSystemLibrary.K2_SetTimerDelegate` (delegate `SDF更新`) 0.01 true))
      (set `self.SDF_Timer` _returnvalue))))

(event `self.ReceiveTick`
  (params (DeltaSeconds :type "Float (single-precision)"))
  (`self.SDF更新`))

(fn `UserConstructionScript`
  (`self.Start Calculate SDF`))